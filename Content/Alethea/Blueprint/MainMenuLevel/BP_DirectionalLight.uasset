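; Directional light actor for the main menu level that animates between two orientations when ChangeDirectionalLight is called.
; A FlipFlop alternately plays and reverses a timeline on successive calls.
; While playing forward or backward, the timeline's curves scale pitch and yaw degree variables, added to fixed base angles with constant roll.
; Tick only caches DeltaSeconds.
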(event `self.ReceiveTick`
  (params (DeltaSeconds :type "Float (single-precision)"))
  (set `self.Delta Seconds` DeltaSeconds))

(event `/Game/Alethea/UI_Widget/UserWidget/BPI_MainMenuLevel.ChangeDirectionalLight`
  (`/Engine/EditorBlueprintResources/StandardMacros.FlipFlop`
    (:`A`
      (bind (_direction _degreey _degreez) (`Timeline|Timeline` :`NewTime` (`self.Delta Seconds`) :!label _label)
        (:`Update`
          (`self.K2_SetActorRotation` (`KismetMathLibrary.MakeRotator` -148.5 (+ (* (`self.DirectionalLightDegreeY`) _degreey) -23.0) (+ (* (`self.DirectionalLightDegreeZ`) _degreez) 124.0))))))
    (:`B`
      (goto _label :!via `Reverse`))))

(fn `UserConstructionScript`)